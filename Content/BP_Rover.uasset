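; BP_Rover runs an automated screenshot loop that repeatedly teledrops, captures a high-res image and counts shots against a maximum.
; After each teleport, a looping timer feeds a velocity check that gates the capture.
; Before each shot, CollapseGraph projects the eight bounds corners of the first "Target"-tagged actor to screen space.
; The min/max results become the 2D box corners on BP_DebugHUD.
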(event `self.ReceiveBeginPlay`
  (bind _outactors (`GameplayStatics.GetAllActorsOfClassWithTag` "/Script/Engine.StaticMeshActor" "Target"))
  (set `self.OriginalLocation` (`SceneComponent.K2_GetComponentLocation` (`Actor.RootComponent` (`|GetArrayItem` _outactors))))
  (`self.StartSequence`))

(event `StartSequence`
  (if (< (`self.ScreenshotCount`) (`self.MaxScreenshots`))
    (set `self.ScreenshotCount` (+ (`self.ScreenshotCount`) 1))
    (`self.Teledrop`)))

(event `Teledrop`
  (bind _returnvalue (`GameplayStatics.GetPlayerController` 0))
  (bind _returnvalue_2 (`KismetMathLibrary.RandomFloatInRange` 20.0 100.0))
  (bind _returnvalue_3 (`KismetMathLibrary.RandomFloatInRange` 0.0 360.0))
  (bind _returnvalue_4 (`KismetMathLibrary.MakeVector` (* (`KismetMathLibrary.DegCos` _returnvalue_3) _returnvalue_2) (* (`KismetMathLibrary.DegSin` _returnvalue_3) _returnvalue_2) 1000.0))
  (bind _outactors (`GameplayStatics.GetAllActorsOfClassWithTag` "/Script/Engine.StaticMeshActor" "Target"))
  (bind _rootcomponent (`Actor.RootComponent` (`|GetArrayItem` _outactors)))
  (`SceneComponent.K2_SetWorldLocation` _rootcomponent (+ (`KismetMathLibrary.MakeVector` 0.0 0.0 1000.0) (`KismetMathLibrary.RandomPointInBoundingBox` (`self.OriginalLocation`) (3000.0 3000.0 100.0))) false true)
  (`KismetSystemLibrary.PrintString` (`KismetStringLibrary.Conv_VectorToString` _returnvalue_4))
  (`SceneComponent.K2_SetWorldLocation` (`self.Cube`) (+ (`SceneComponent.K2_GetComponentLocation` _rootcomponent) _returnvalue_4) false true)
  (`KismetSystemLibrary.Delay` 1.0)
  (`|ExecutionSequence`
    (:`then_0`
      (goto _label :!via `Open`))
    (:`then_1`
      (bind _returnvalue_5 (`KismetSystemLibrary.K2_SetTimerDelegate` (delegate `CheckVelocity`) 0.1 true))
      (set `self.CheckTimerHandle` _returnvalue_5))))

(event `CheckVelocity`
  (bind _returnvalue (`GameplayStatics.GetPlayerController` 0))
  (`/Engine/EditorBlueprintResources/StandardMacros.Gate` true :!label _label
    (:`Exit`
      (if (< (`KismetMathLibrary.VSize` (`SceneComponent.GetComponentVelocity` (`self.Cube`))) (`self.VelocityThreshhold`))
        (set `self.StableTime` (+ (`self.StableTime`) 0.1))
        (else
          (set `self.StableTime` 0.0)))
      (if (>= (`self.StableTime`) (`self.StableDuration`))
        (`|ExecutionSequence`
          (:`then_0`
            (goto _label :!via `Close`))
          (:`then_1`
            (cast `/Game/BP_CineCameraActor` (`ChildActorComponent.ChildActor` (`self.BP_CineCameraActor`)))
            (bind _outactors (`GameplayStatics.GetAllActorsWithTag` "Target"))
            (bind _output (`|GetArrayItem` _outactors))
            (bind (_origin _boxextent) (`self.GetActorBounds` _output false false))
            (bind _x (.x _boxextent))
            (bind _y (.y _boxextent))
            (bind _z (.z _boxextent))
            (bind _returnvalue_2 (`self.K2_GetActorRotation` _output))
            (bind _returnvalue_3 (+ _origin (`KismetMathLibrary.GreaterGreater_VectorRotator` (`KismetMathLibrary.MakeVector` _x _y _z) _returnvalue_2)))
            (`KismetSystemLibrary.PrintString` (`KismetStringLibrary.Conv_VectorToString` _returnvalue_3))
            (bind _outactors_2 (`GameplayStatics.GetAllActorsOfClass` "/Game/BP_DebugHUD.BP_DebugHUD_C"))
            (bind (_x_2 _y_2) (`KismetMathLibrary.BreakVector2D` (`GameplayStatics.ProjectWorldToScreen` _returnvalue _returnvalue_3)))
            (bind _x_3 (.x (`KismetMathLibrary.NegateVector` _boxextent)))
            (bind _y_3 (.y (`KismetMathLibrary.NegateVector` _boxextent)))
            (bind _z_2 (.z (`KismetMathLibrary.NegateVector` _boxextent)))
            (bind (_x_4 _y_4) (`KismetMathLibrary.BreakVector2D` (`GameplayStatics.ProjectWorldToScreen` _returnvalue (+ _origin (`KismetMathLibrary.GreaterGreater_VectorRotator` (`KismetMathLibrary.MakeVector` _x_3 _y _z) _returnvalue_2)))))
            (bind (_x_5 _y_5) (`KismetMathLibrary.BreakVector2D` (`GameplayStatics.ProjectWorldToScreen` _returnvalue (+ _origin (`KismetMathLibrary.GreaterGreater_VectorRotator` (`KismetMathLibrary.MakeVector` _x _y_3 _z) _returnvalue_2)))))
            (bind (_x_6 _y_6) (`KismetMathLibrary.BreakVector2D` (`GameplayStatics.ProjectWorldToScreen` _returnvalue (+ _origin (`KismetMathLibrary.GreaterGreater_VectorRotator` (`KismetMathLibrary.MakeVector` _x_3 _y_3 _z) _returnvalue_2)))))
            (bind (_x_7 _y_7) (`KismetMathLibrary.BreakVector2D` (`GameplayStatics.ProjectWorldToScreen` _returnvalue (+ _origin (`KismetMathLibrary.GreaterGreater_VectorRotator` (`KismetMathLibrary.MakeVector` _x _y _z_2) _returnvalue_2)))))
            (bind (_x_8 _y_8) (`KismetMathLibrary.BreakVector2D` (`GameplayStatics.ProjectWorldToScreen` _returnvalue (+ _origin (`KismetMathLibrary.GreaterGreater_VectorRotator` (`KismetMathLibrary.MakeVector` _x_3 _y _z_2) _returnvalue_2)))))
            (bind (_x_9 _y_9) (`KismetMathLibrary.BreakVector2D` (`GameplayStatics.ProjectWorldToScreen` _returnvalue (+ _origin (`KismetMathLibrary.GreaterGreater_VectorRotator` (`KismetMathLibrary.MakeVector` _x _y_3 _z_2) _returnvalue_2)))))
            (bind (_x_10 _y_10) (`KismetMathLibrary.BreakVector2D` (`GameplayStatics.ProjectWorldToScreen` _returnvalue (+ _origin (`KismetMathLibrary.GreaterGreater_VectorRotator` (`KismetMathLibrary.MakeVector` _x_3 _y_3 _z_2) _returnvalue_2)))))
            (bind _output_2 (`|GetArrayItem` _outactors_2))
            (set `/Game/BP_DebugHUD.LeftCorner` (`KismetMathLibrary.MakeVector2D` (`KismetMathLibrary.FMin` _x_2 _x_4 _x_5 _x_6 _x_7 _x_8 _x_9 _x_10) (`KismetMathLibrary.FMin` _y_2 _y_4 _y_5 _y_6 _y_7 _y_8 _y_9 _y_10)) _output_2)
            (set `/Game/BP_DebugHUD.RightCorner` (`KismetMathLibrary.MakeVector2D` (`KismetMathLibrary.FMax` _x_2 _x_4 _x_5 _x_6 _x_7 _x_8 _x_9 _x_10) (`KismetMathLibrary.FMax` _y_2 _y_4 _y_5 _y_6 _y_7 _y_8 _y_9 _y_10)) _output_2)
            (`AutomationBlueprintFunctionLibrary.TakeHighResScreenshot` 1280 1280 "" null)
            (`KismetSystemLibrary.Delay` 1.0)
            (`self.StartSequence`)))))))

(fn `NewFunction`)

(fn `UserConstructionScript`)