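; Cine camera actor with get and set functions for position and a ReadyForCapture flag, apparently meant to be driven externally.
; SetPos ignores its input location except for printing it, instead offsetting actor and camera component by a sine of real-time partial seconds.
; It then aims the camera at the first actor tagged "Target".
; BeginPlay and Tick do nothing, and leftover positioning and look-at nodes are disconnected.
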(event `self.ReceiveTick`
  (params (DeltaSeconds :type "Float (single-precision)")))

(fn `GetPos`
  (returns (Loc :type "Vector Structure"))
  (return (`self.K2_GetActorLocation`)))

(fn `GetReady`
  (returns (Ready :type Boolean))
  (return (`self.ReadyForCapture`)))

(fn `SetPos`
  (params (NewLoc :type "Vector Structure"))
  (bind _cameracomponent (`self.CameraComponent`))
  (bind _returnvalue (* (`KismetMathLibrary.DegSin` (`.PartialSeconds` (`GameplayStatics.GetAccurateRealTime`))) 1000.0))
  (bind _returnvalue_2 (+ (`self.K2_GetActorLocation`) (`KismetMathLibrary.MakeVector` _returnvalue _returnvalue _returnvalue)))
  (`self.K2_SetActorLocation` _returnvalue_2 false true)
  (`SceneComponent.K2_SetWorldLocation` _cameracomponent _returnvalue_2 false true)
  (`KismetSystemLibrary.PrintString` (`KismetStringLibrary.Conv_VectorToString` NewLoc))
  (bind _outactors (`GameplayStatics.GetAllActorsWithTag` "Target"))
  (`SceneComponent.K2_SetWorldRotation` _cameracomponent (`KismetMathLibrary.FindLookAtRotation` (`SceneComponent.K2_GetComponentLocation` _cameracomponent) (`self.K2_GetActorLocation` (`|GetArrayItem` _outactors))) false false)
  (return))

(fn `SetReady`
  (params (Ready :type Boolean))
  (set `self.ReadyForCapture` Ready)
  (return))

(fn `UserConstructionScript`)